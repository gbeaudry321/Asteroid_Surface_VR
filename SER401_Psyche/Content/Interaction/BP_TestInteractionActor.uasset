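; BP_TestInteractionActor is a test interactable that opens a carousel UI when the player interacts with it.
; Focus toggles custom depth rendering on its Cube, and an InteractionWidget reference is exposed through a getter.
; Interact creates and activates WBP_IP_Carousel_Template in the viewport, switches player 0 to UI-only input with a visible cursor, and returns true.
; LookAt returns an empty string.
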(event EventInterfaceToggleFocus
  (params (Focus :type Boolean))
  (Rendering|SetRenderCustomDepth (Variables|Default|GetCube) Focus))

(fn ConstructionScript)

(fn GetInteractionWidgetRef
  (return (Variables|Default|GetInteraction_Widget)))

(fn Interact
  (params (Interactor :type Actor%20Object%20Reference))
  (bind _returnvalue (Game|GetPlayerController 0))
  (bind _returnvalue_2 (UserInterface|CreateWidget "/Game/UI/InfoPoints/WBP_IP_Carousel_Template.WBP_IP_Carousel_Template_C"))
  (UserInterface|Viewport|AddtoViewport _returnvalue_2 0)
  (Class|CommonActivatableWidget|ActivateWidget _returnvalue_2)
  (Input|SetInputModeUIOnly _returnvalue 0 "DoNotLock" false)
  (Variables|/Script/Engine.PlayerController|SetbShowMouseCursor _returnvalue true)
  (return true))

(fn Lookat
  (return ""))