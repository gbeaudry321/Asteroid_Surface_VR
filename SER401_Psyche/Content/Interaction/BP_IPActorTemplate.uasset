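; Template info-point actor that shows a marker when a character is nearby and opens a carousel widget when interacted with.
; Collision overlaps toggle the InfoPoint widget's visibility, and the BI_Interaction focus event outlines the Cube through custom depth.
; Interact creates and activates WBP_IP_Carousel_Template, then switches to UI-only input with the mouse cursor shown.
; It also returns its prompt widget through GetInteractionWidgetRef, while LookAt returns empty text.
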(event OnComponentBeginOverlap(Collision)
  (params (OverlappedComponent :type Primitive%20Component%20Object%20Reference) (OtherActor :type Actor%20Object%20Reference) (OtherComp :type Primitive%20Component%20Object%20Reference) (OtherBodyIndex :type Integer) (bFromSweep :type Boolean) (SweepResult :type Hit%20Result%20Structure%20%28by%20ref%29))
  ;[1 1 1] Make info point visible when player overlaps
  (Utilities|Casting|CastToCharacter OtherActor)
  (CallFunction|ChangeWidgetVisibility true))

(event OnComponentEndOverlap(Collision)
  (params (OverlappedComponent :type Primitive%20Component%20Object%20Reference) (OtherActor :type Actor%20Object%20Reference) (OtherComp :type Primitive%20Component%20Object%20Reference) (OtherBodyIndex :type Integer))
  ;[1 1 1] Make info point not visible when player leaves overlap
  (Utilities|Casting|CastToCharacter OtherActor)
  (CallFunction|ChangeWidgetVisibility false))

(event Custom|ChangeWidgetVisibility
  (params (isVisible :type Boolean))
  ;[1 1 1] Change the visibility of the infopoint widget. Called in Begin/End overlap
  (Rendering|SetVisibility (Variables|Default|GetInfoPoint) isVisible false))

(event EventBeginPlay
  ;[1 1 1] InfoPoint not visible on start
  (Rendering|SetVisibility (Variables|Default|GetInfoPoint) false false))

(event EventInterfaceToggleFocus
  (params (Focus :type Boolean))
  ;[1 1 1] Uses the Blueprint Interface BI_Interaction function Toggle Focus to determine if the player is in range of and focused on the actor. Makes the outline visible if true.
  ;
  ; See the Interfaces section in the My Blueprint tab on the right for further functionality
  (Rendering|SetRenderCustomDepth (Variables|Default|GetCube) Focus))

(fn ConstructionScript)

(fn GetInteractionWidgetRef
  ;[1 1 1] Interaction prompt widget that appears (Content>Interaction>WB_Interation_Prompt)
  (return (Variables|Default|GetInteraction_Widget)))

(fn Interact
  (params (Interactor :type Actor%20Object%20Reference))
  (bind _returnvalue (Game|GetPlayerController 0))
  ;[1 1 1] If the player calls the Interact function, the specified widget (WBP_IP_Carousel_Template in this case) is added to the player's viewport, activated, and Input mode is set to UI only so the player can interact with the widget.
  ; See the InfoPoint Interaction of the BP_FirstPersonCharacter for an example. Content>Characters>FirstPerson>Blueprints
  (bind _returnvalue_2 (UserInterface|CreateWidget "/Game/UI/InfoPoints/WBP_IP_Carousel_Template.WBP_IP_Carousel_Template_C"))
  (UserInterface|Viewport|AddtoViewport _returnvalue_2 0)
  (Class|CommonActivatableWidget|ActivateWidget _returnvalue_2)
  (Input|SetInputModeUIOnly _returnvalue 0 "DoNotLock" false)
  (Variables|/Script/Engine.PlayerController|SetbShowMouseCursor _returnvalue true)
  (return false))

(fn Lookat
  (return ""))