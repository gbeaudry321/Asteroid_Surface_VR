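; Ship actor that acts as an interactable storage container and navigation target for the player.
; On BeginPlay it writes its location to the first-person character's NavPoint, a one-time snapshot.
; Interactwith has the player controller's HUD show its InventorySystem as a container, while LookAt returns an empty string.
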(event EventBeginPlay
  (bind _asbp_first_person_character (Utilities|Casting|CastToBP_FirstPersonCharacter (Game|GetPlayerCharacter 0)))
  (Variables|/Game/Characters/FirstPerson/Blueprints/BP_FirstPersonCharacter.BP_FirstPersonCharacter_C|SetNavPoint _asbp_first_person_character (Transformation|GetActorLocation)))

(event EventInteractwith
  (params (PlayerCharacter :type BP%20First%20Person%20Character%20Object%20Reference))
  (bind _asbp_first_person_player_controller (Utilities|Casting|CastToBP_FirstPersonPlayerController (Game|GetPlayerController 0)))
  (Default|ShowContainer (Variables|/Game/Characters/FirstPerson/Blueprints/BP_FirstPersonPlayerController.BP_FirstPersonPlayerController_C|GetHUD _asbp_first_person_player_controller) (Variables|Default|GetInventorySystem)))

(fn ConstructionScript)

(fn Lookat
  (return ""))