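; Satellite actor that moves its static mesh along a looping spline at a set speed.
; Each Tick advances the distance, wraps it to zero at the spline's end, and takes location, roll and offset yaw from the spline while keeping the mesh's pitch.
; It also writes the current local-space spline position to SatPoint on the first-person character and VR pawn, whichever the player controls.
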(event EventTick
  (params (DeltaSeconds :type Float%20%28single-precision%29))
  (Utilities|FlowControl|Sequence
    (:then_0
      (Variables|Default|Setdistance (+ (* DeltaSeconds (Variables|Default|Getspeed)) (Variables|Default|Getdistance)))
      (Transformation|SetRelativeTransform (Variables|Default|GetStaticMesh) (Math|Transform|MakeTransform (.location (Spline|GetTransformatDistanceAlongSpline (Variables|Default|GetSpline) (Variables|Default|Getdistance) "Local" false)) (Math|Rotator|MakeRotator (.roll (.rotation (Spline|GetTransformatDistanceAlongSpline (Variables|Default|GetSpline) (Variables|Default|Getdistance) "Local" false))) (.pitch (.rotation (Transformation|GetRelativeTransform (Variables|Default|GetStaticMesh)))) (+ (.yaw (.rotation (Spline|GetTransformatDistanceAlongSpline (Variables|Default|GetSpline) (Variables|Default|Getdistance) "Local" false))) -9e+01)) (Variables|/Script/Engine.SceneComponent|GetRelativeScale3D (Variables|Default|GetStaticMesh))) false false)
      (if (> (Variables|Default|Getdistance) (Spline|GetSplineLength (Variables|Default|GetSpline)))
        (Variables|Default|Setdistance 0.0)))
    (:then_1
      (bind _asbp_first_person_character (Utilities|Casting|CastToBP_FirstPersonCharacter (Game|GetPlayerCharacter 0)))
      (Variables|/Game/Characters/FirstPerson/Blueprints/BP_FirstPersonCharacter.BP_FirstPersonCharacter_C|SetSatPoint _asbp_first_person_character (.location (Spline|GetTransformatDistanceAlongSpline (Variables|Default|GetSpline) (Variables|Default|Getdistance) "Local" false))))
    (:then_2
      (bind _asvrpawn (Utilities|Casting|CastToVRPawn (Game|Player|GetPlayerPawn 0)))
      (Variables|/Game/VRTemplate/Blueprints/VRPawn.VRPawn_C|SetSatPoint _asvrpawn (.location (Spline|GetTransformatDistanceAlongSpline (Variables|Default|GetSpline) (Variables|Default|Getdistance) "Local" false))))))

(fn ConstructionScript)